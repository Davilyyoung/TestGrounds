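; BP_Tile is a terrain segment for an infinite map, exposing an arrow transform as its attach location.
; Its barrier wall starts locked and red, turning green and passable while the player overlaps the locking volume.
; When the player leaves that volume, the wall relocks and BP_GameMode spawns another tile.
; The tile destroys itself when the player enters its destroy volume.
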(event OnComponentBeginOverlap(LockingValume)
  (params (OverlappedComponent :type Primitive%20Component%20Object%20Reference) (OtherActor :type Actor%20Object%20Reference) (OtherComp :type Primitive%20Component%20Object%20Reference) (OtherBodyIndex :type Integer) (bFromSweep :type Boolean) (SweepResult :type Hit%20Result%20Structure%20%28by%20ref%29))
  ;[1 1 1] Wall Locking
  (Utilities|IsPlayerActor OtherActor)
  (CallFunction|Unlock))

(event OnComponentEndOverlap(LockingValume)
  (params (OverlappedComponent :type Primitive%20Component%20Object%20Reference) (OtherActor :type Actor%20Object%20Reference) (OtherComp :type Primitive%20Component%20Object%20Reference) (OtherBodyIndex :type Integer))
  ;[1 1 1] Wall Locking
  (Utilities|IsPlayerActor OtherActor)
  (CallFunction|Lock)
  ;[1 1 1] Infinite Map
  (bind _asbp_game_mode (Utilities|Casting|CastToBP_GameMode (Game|GetGameMode)))
  (Default|SpawnTile _asbp_game_mode))

(event OnComponentBeginOverlap(DestroyValume)
  (params (OverlappedComponent :type Primitive%20Component%20Object%20Reference) (OtherActor :type Actor%20Object%20Reference) (OtherComp :type Primitive%20Component%20Object%20Reference) (OtherBodyIndex :type Integer) (bFromSweep :type Boolean) (SweepResult :type Hit%20Result%20Structure%20%28by%20ref%29))
  (Utilities|IsPlayerActor OtherActor)
  (Actor|DestroyActor))

(event EventBeginPlay
  (CallFunction|Lock))

(fn ConstructionScript)

(fn GetAttacthLocation
  (return (Transformation|GetWorldTransform (Variables|Default|GetArrow))))

(fn Unlock
  (bind _lockwall (Variables|Default|GetLockWall))
  (Collision|SetCollisionEnabled _lockwall "NoCollision")
  (Rendering|Material|SetMaterial _lockwall 0 "/Game/Static/Geometry/Meshes/MT_BarrierGreen_Inst.MT_BarrierGreen_Inst"))

(fn Lock
  (bind _lockwall (Variables|Default|GetLockWall))
  (Collision|SetCollisionEnabled _lockwall "QueryAndPhysics")
  (Rendering|Material|SetMaterial _lockwall 0 "/Game/Static/Geometry/Meshes/MT_BarrierRed_Inst.MT_BarrierRed_Inst"))