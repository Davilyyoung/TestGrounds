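; AI controller for NPCs that runs a behavior tree and tracks a perceived target.
; On BeginPlay it sets up the BB_PatolData blackboard and starts the BTE_Base behavior tree.
; AI perception updates write any sensed actor lacking the "Enemy" tag to the EnemyKey blackboard value and clear it when sensing fails.
; Debug prints report when a target is found or lost.
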(event OnTargetPerceptionUpdated(AIPerception)
  (params (Actor :type Actor%20Object%20Reference) (Stimulus :type AI%20Stimulus%20Structure))
  (bind _blackboard_component (Variables|Default|GetBlackboard%20Component))
  (bind _enemykey (Variables|Default|GetEnemyKey))
  ;[1 1 1] Find Player
  (if (not (Actor|ActorHasTag Actor "Enemy"))
    (if (.bSuccessfullySensed (Utilities|Struct|BreakAIStimulus Stimulus))
      (AI|Components|Blackboard|SetValueasObject _blackboard_component _enemykey Actor)
      (Development|PrintString "Find Player")
      (else
        (AI|Components|Blackboard|ClearValue _blackboard_component _enemykey)
        (Development|PrintString "No Target")))))

(event EventBeginPlay
  ;[1 1 1] Run BT
  (bind _blackboardcomponent (Class|AIController|UseBlackboard "/Game/Dynamic/NPC/Behaviour/AI_Behaviour/BB_PatolData.BB_PatolData"))
  (AI|RunBehaviorTree "/Game/Dynamic/NPC/Behaviour/AI_Behaviour/BTE_Base.BTE_Base")
  (Variables|Default|SetBlackboard%20Component _blackboardcomponent))

(fn ConstructionScript)