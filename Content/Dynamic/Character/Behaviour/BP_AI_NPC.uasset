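; AI controller for NPCs that starts behavior tree BTE_Base with blackboard BB_PatolData on BeginPlay.
; AI perception updates feed the blackboard's EnemyKey, storing any successfully sensed actor that lacks the "Enemy" tag as the target.
; When sensing of such an actor fails, the key is cleared without checking which actor it currently holds.
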(event OnTargetPerceptionUpdated(AIPerception)
  (params (Actor :type Actor%20Object%20Reference) (Stimulus :type AI%20Stimulus%20Structure))
  ;[1 1 1] Find Player
  (CallFunction|UpdateBlackboardEnemyKey Actor Actor Stimulus))

(event EventBeginPlay
  ;[1 1 1] Run BT
  (bind _blackboardcomponent (Class|AIController|UseBlackboard "/Game/Dynamic/Character/Behaviour/AI_Behaviour/BB_PatolData.BB_PatolData"))
  (AI|RunBehaviorTree "/Game/Dynamic/Character/Behaviour/AI_Behaviour/BTE_Base.BTE_Base")
  (Variables|Default|SetBlackboard%20Component _blackboardcomponent))

(fn ConstructionScript)

(fn UpdateBlackboardEnemyKey
  (params (self2 :type Actor%20Object%20Reference) (ObjectValue :type Object%20Object%20Reference) (AIStimulus :type AI%20Stimulus%20Structure%20%28by%20ref%29))
  (bind _blackboard_component (Variables|Default|GetBlackboard%20Component))
  (bind _enemykey (Variables|Default|GetEnemyKey))
  (if (not (Actor|ActorHasTag self2 "Enemy"))
    (if (.bSuccessfullySensed (Utilities|Struct|BreakAIStimulus AIStimulus))
      (AI|Components|Blackboard|SetValueasObject _blackboard_component _enemykey ObjectValue)
      (else
        (AI|Components|Blackboard|ClearValue _blackboard_component _enemykey)))))